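; BP_SaveGameSystem is a save object that carries day progress between the game instance and storage: current and start-of-day parameters, the current event and the day's events.
; SaveGame copies these values from the passed game instance into the object, but its SaveGameToSlot node is unconnected, so writing to disk does not happen here.
; LoadGame reads the "AutoSave" slot, casts it to this class and copies the values back into the game instance.
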(event `SaveGame`
  (params (GameInst :type "/Game/Blueprints/GI_GameInstance Object Reference"))
  (set `self.Parametrs at Start Day` (`/Game/Blueprints/GI_GameInstance.Parametrs_AtStartDay` GameInst))
  (set `self.Parametrs` (`/Game/Blueprints/GI_GameInstance.Parametrs` GameInst))
  (set `self.Current Event` (`/Game/Blueprints/GI_GameInstance.CurrentEvent` GameInst))
  (set `self.Events for Current Day` (`/Game/Blueprints/GI_GameInstance.EventsForCurrentDay` GameInst)))

(event `LoadGame`
  (params (GameInsr :type "/Game/Blueprints/GI_GameInstance Object Reference"))
  (bind _returnvalue (`GameplayStatics.LoadGameFromSlot` "AutoSave"))
  (bind _asbp_save_game_system (cast `/Game/Blueprints/BP_SaveGameSystem` _returnvalue))
  (set `/Game/Blueprints/GI_GameInstance.CurrentEvent` (`/Game/Blueprints/BP_SaveGameSystem.Current Event` _asbp_save_game_system) GameInsr)
  (set `/Game/Blueprints/GI_GameInstance.EventsForCurrentDay` (`/Game/Blueprints/BP_SaveGameSystem.Events for Current Day` _asbp_save_game_system) GameInsr)
  (set `/Game/Blueprints/GI_GameInstance.Parametrs` (`/Game/Blueprints/BP_SaveGameSystem.Parametrs` _asbp_save_game_system) GameInsr)
  (set `/Game/Blueprints/GI_GameInstance.Parametrs_AtStartDay` (`/Game/Blueprints/BP_SaveGameSystem.Parametrs at Start Day` _asbp_save_game_system) GameInsr))