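; Main game mode that runs the day loop of a narrative game about receiving visitors, letters and writing replies.
; Each day it gathers events and letters from DataTables and drives UI widgets through letters, visits and day end, skipping visits whose required past events are missing.
; Visit outcomes adjust clamped Royal, Shadow and Holy stats in the game instance, record past events, and trigger an alarm when a stat hits zero.
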(event `self.ReceiveBeginPlay`
  (`self.NewDay`)
  (bind _returnvalue (`AddComponent|NODE_AddAudioComponent-1`))
  (set `self.SFX_Buttons` _returnvalue)
  (bind _returnvalue_2 (`AddComponent|NODE_AddAudioComponent-2`))
  (set `self.SFX_Game` _returnvalue_2)
  (bind _returnvalue_3 (`AddComponent|NODE_AddAudioComponent-5`))
  (set `self.SFX_Letters` _returnvalue_3)
  (bind _returnvalue_4 (`AddComponent|NODE_AddAudioComponent-6`))
  (set `self.SFX_Doors` _returnvalue_4)
  (bind _returnvalue_5 (`AddComponent|NODE_AddAudioComponent-7`))
  (set `self.SFX_Alarm` _returnvalue_5))

(event `CheckAfterNewDay`
  (if (== (`.Day_11_FD3FEA414E56BE98A9503E87627CA723` (break `/Game/Blueprints/DataTable/Parametrs` (`self.GetParametrs`))) 1)
    (bind _widgetobj (`self.AddWidgetToVieport` "/Game/UI/WB_LastLetter.WB_LastLetter_C"))
    (bind _aswb_last_letter (cast `/Game/UI/WB_LastLetter` _widgetobj))
    (set `/Game/UI/WB_LastLetter.IfFirstShow` true _aswb_last_letter)
    (else
      (`self.SetupLettersForDay`)
      (`self.ReadLetters`))))

(event `WriteLetter?`
  (bind _as_wb_visit (`self.As WB Visit`))
  (if (`self.Is Writing?`)
    (`/Game/UI/WB_Visit.WritingLetter` _as_wb_visit)
    (else
      (`/Game/UI/WB_Visit.EndVisitWithoutWritting` _as_wb_visit)
      (`KismetSystemLibrary.Delay` 1.7)
      (`self.EndVisit` false))))

(event `ChooseAdress`
  (params (FinalResult :type String))
  (bind _returnvalue (`|CreateWidget` "/Game/UI/WB_ChoseAdressee.WB_ChoseAdressee_C"))
  (set `self.WBAdress` _returnvalue)
  (`/Game/UI/WB_ChoseAdressee.InitCountAdressats` _returnvalue FinalResult)
  (`UserWidget.AddToViewport` _returnvalue 0)
  (add `/Game/UI/WB_ChoseAdressee.EndVisit` _returnvalue (delegate `EndVisi`)))

(event `EndVisi`
  (params (AfterEffects :type "/Game/Blueprints/DataTable/AfterEffectsForAdressats Structure"))
  (`self.EndVisit` (`self.Is Writing?`) AfterEffects))

(event `AfterVisit`
  (bind _sfx_letters (`self.SFX_Letters`))
  (if (`self.IsAlarm`)
    (`self.SetSFX` 2 _sfx_letters "SendLetter")
    (else
      (`self.SetSFX` 1 _sfx_letters "SendLetter")))
  (`KismetSystemLibrary.Delay` 2.0)
  (`Widget.RemoveFromParent` (`self.WBAdress`))
  (`self.CheckEndVisits?`))

(fn `AddWidgetToVieport`
  (params (WidgetClass :type "UserWidget Class Reference"))
  (returns (WidgetObj :type "UserWidget Object Reference"))
  (bind _returnvalue (`|CreateWidget` WidgetClass))
  (`UserWidget.AddToViewport` _returnvalue 0)
  (return _returnvalue))

(fn `CheckEndVisits?`
  (bind _gameinst (`self.GameInst`))
  (if (>= (`/Game/Blueprints/GI_GameInstance.CurrentEvent` _gameinst) (`KismetArrayLibrary.Array_Length` (`/Game/Blueprints/GI_GameInstance.EventsForCurrentDay` _gameinst)))
    (`self.EndDay`)
    (else
      (`self.NewVisits`))))

(fn `CheckLettersAtDay`)

(fn `CheckParamZero`
  (bind (_parametrs_royal _parametrs_shadow _parametrs_holy) (break `/Game/Blueprints/DataTable/Parametrs` (`self.GetParametrs`)))
  (bind (_parametrs_royal_2 _parametrs_shadow_2 _parametrs_holy_2) (break `/Game/Blueprints/DataTable/Parametrs` (`self.GetParametrs`)))
  (if (`self.IsAlarm`)
    (if (not (== _parametrs_royal 0))
      (set `self.AlarmRoyal` false)
      (if (not (== _parametrs_shadow 0))
        (set `self.AlarmShadow` false)
        (if (not (== _parametrs_holy 0))
          (set `self.AlarmHoly` false)
          (if (`self.AlarmRoyal`)
            _
            (elif (`self.AlarmShadow`)
              _
              (elif (not (`self.AlarmHoly`))
                (`self.SetSFX` 0 (`self.SFX_Alarm`) "Alarm")
                (set `self.IsAlarm` false)))))))
    (else
      (`|ExecutionSequence`
        (:`then_0`
          (if (== _parametrs_royal_2 0)
            (set `self.AlarmRoyal` true)
            (`self.SetSFX` 1 (`self.SFX_Alarm`) "Alarm" :!label _label)
            (set `self.IsAlarm` true)))
        (:`then_1`
          (if (== _parametrs_shadow_2 0)
            (set `self.AlarmShadow` true)
            (goto _label)))
        (:`then_2`
          (if (== _parametrs_holy_2 0)
            (set `self.AlarmHoly` true)
            (goto _label)))))))

(fn `Death`
  (`self.AddWidgetToVieport` "/Game/UI/WB_Ending.WB_Ending_C"))

(fn `EndDay`
  (bind _widgetobj (`self.AddWidgetToVieport` "/Game/UI/WB_EndDay.WB_EndDay_C"))
  (bind _aswb_end_day (cast `/Game/UI/WB_EndDay` _widgetobj))
  (`/Game/UI/WB_Parametrs.UpdateParametrs` (`/Game/UI/WB_EndDay.WB_Parametrs` _aswb_end_day)))

(fn `EndVisit`
  (params (`Write?` :type Boolean) (AfterEffects :type "/Game/Blueprints/DataTable/AfterEffectsForAdressats Structure"))
  (bind (_royal _shadow _holy _condition _finalresult) (break `/Game/Blueprints/DataTable/AfterEffectsForAdressats` AfterEffects))
  (if `Write?`
    (`self.NewMacro` _royal _shadow _holy _finalresult)
    (`/Engine/EditorBlueprintResources/StandardMacros.IncrementInt` (`/Game/Blueprints/GI_GameInstance.CurrentEvent` (`self.GameInst`))
      (:`  `
        (`self.AfterVisit`)))
    (else
      (bind _returnvalue (`|GetDataTableRow` "/Game/Blueprints/DataTable/Events.Events" (`self.GetCurrentEventRow`))
        (:`then`
          (bind (_royal_2 _shadow_2 _holy_2 _finalresult_2) (break `/Game/Blueprints/DataTable/AfterEffects` (`.ParamsWithoutLetter_39_AB3DC4E645F88A52087B6BA95C372CB8` (break `/Game/Blueprints/DataTable/EventForDay` _returnvalue))))
          (`self.NewMacro` _royal_2 _shadow_2 _holy_2 _finalresult_2)
          (`/Engine/EditorBlueprintResources/StandardMacros.IncrementInt` (`/Game/Blueprints/GI_GameInstance.CurrentEvent` (`self.GameInst`))
            (:`  `
              (`self.CheckEndVisits?`))))))))

(fn `GetCurrentEventRow`
  (returns (Output :type Name))
  (bind _gameinst (`self.GameInst`))
  (return (`|GetArrayItem` (`/Game/Blueprints/GI_GameInstance.EventsForCurrentDay` _gameinst) (`/Game/Blueprints/GI_GameInstance.CurrentEvent` _gameinst))))

(fn `GetParametrs`
  (returns (Parametrs :type "/Game/Blueprints/DataTable/Parametrs Structure"))
  (return (`/Game/Blueprints/GI_GameInstance.Parametrs` (`self.GameInst`))))

(fn `NewDay`
  (`self.SetSFX` 0 (`self.SFX_Game`) "TimeOfDay")
  (bind _widgetobj (`self.AddWidgetToVieport` "/Game/UI/WB_NewDay.WB_NewDay_C"))
  (bind _aswb_new_day (cast `/Game/UI/WB_NewDay` _widgetobj))
  (`/Game/UI/WB_NewDay.Begin` _aswb_new_day (`.Day_11_FD3FEA414E56BE98A9503E87627CA723` (break `/Game/Blueprints/DataTable/Parametrs` (`self.GetParametrs`))))
  (`self.SetupEventsForDay`)
  (set `/Game/Blueprints/GI_GameInstance.Parametrs_AtStartDay` (`self.GetParametrs`) (`self.GameInst`)))

(fn `NewVisits`
  (bind _as_wb_visit (`self.As WB Visit`))
  (`/Engine/EditorBlueprintResources/StandardMacros.IsValid` _as_wb_visit
    (:`Is Valid`
      (`Widget.SetVisibility` _as_wb_visit "Visible"))
    (:`Is Not Valid`
      (bind _returnvalue (`|CreateWidget` "/Game/UI/WB_Visit.WB_Visit_C"))
      (`UserWidget.AddToViewport` _returnvalue 0)
      (bind _output_get (set `self.As WB Visit` _returnvalue))
      (add `/Game/UI/WB_Visit.WriteLetter` _output_get (`|CreateDelegate` :!event `WriteLetter?`))
      (add `/Game/UI/WB_Visit.ChoseAdress` (`self.As WB Visit`) (`|CreateDelegate` :!event `ChooseAdress`))))
  (bind _returnvalue_2 (`|GetDataTableRow` "/Game/Blueprints/DataTable/Events.Events" (`self.GetCurrentEventRow`))
    (:`then`
      (bind (_reccondition _nameevent _namevisiter _text _timeofday _day _iswriting_) (break `/Game/Blueprints/DataTable/EventForDay` _returnvalue_2))
      (if (`KismetArrayLibrary.Array_IsEmpty` _reccondition)
        (`self.SetSFX` (+ (`KismetMathLibrary.Conv_ByteToInt` _timeofday) 1) (`self.SFX_Game`) "TimeOfDay" :!label _label)
        (set `self.Is Writing?` _iswriting_)
        (`/Game/UI/WB_Visit.VisitBegin` (`self.As WB Visit`) _timeofday _namevisiter _text)
        (else
          (for _array_element _reccondition
            (if (== (`KismetArrayLibrary.Array_Find` (`.PastEvents_16_FE7FEA354431C0A8972FC8BF01629BBB` (break `/Game/Blueprints/DataTable/Parametrs` (`/Game/Blueprints/GI_GameInstance.Parametrs` (`self.GameInst`)))) _array_element) -1)
              (`/Engine/EditorBlueprintResources/StandardMacros.IncrementInt` (`/Game/Blueprints/GI_GameInstance.CurrentEvent` (`self.GameInst`))
                (:`  `
                  (`self.CheckEndVisits?`)))
              (else
                (goto _label)))))))))

(fn `ReadLetters`
  (if (`KismetArrayLibrary.Array_IsEmpty` (`self.LettersForCurrentDay`))
    (`self.NewVisits`)
    (else
      (bind _returnvalue (`|CreateWidget` "/Game/UI/WB_ReadLetter.WB_ReadLetter_C"))
      (`UserWidget.AddToViewport` _returnvalue 0))))

(fn `SetParametrs`
  (params (Parametrs :type "/Game/Blueprints/DataTable/Parametrs Structure"))
  (bind (_royal _shadow _holy _day _pastevents) (break `/Game/Blueprints/DataTable/Parametrs` Parametrs))
  (set `/Game/Blueprints/GI_GameInstance.Parametrs` (make `/Game/Blueprints/DataTable/Parametrs` (`KismetMathLibrary.Clamp` _royal 0 4) (`KismetMathLibrary.Clamp` _shadow 0 4) (`KismetMathLibrary.Clamp` _holy 0 4) _day _pastevents) (`self.GameInst`))
  (`/Game/UI/WB_Visit.UpdateParam` (`self.As WB Visit`))
  (`self.CheckParamZero`))

(fn `SetSFX`
  (params (Int :type Integer) (AudioComp :type "AudioComponent Object Reference") (Param :type Name))
  (`/Engine/EditorBlueprintResources/StandardMacros.IsValid` AudioComp
    (:`Is Valid`
      (`AudioComponent.SetIntParameter` AudioComp Param Int)
      (`AudioComponent.Play` AudioComp 0.0))))

(fn `SetupEventsForDay`
  (bind _gameinst (`self.GameInst`))
  (`KismetArrayLibrary.Array_Clear` (`/Game/Blueprints/GI_GameInstance.EventsForCurrentDay` (`self.GameInst`)))
  (bind _outrownames (`DataTableFunctionLibrary.GetDataTableRowNames` "/Game/Blueprints/DataTable/Events.Events"))
  (for _array_element _outrownames
    (bind _returnvalue (`|GetDataTableRow` "/Game/Blueprints/DataTable/Events.Events" _array_element)
      (:`then`
        (if (== (`.Day_19_21EE1D6B4EF31695295742ABEA97A2BA` (break `/Game/Blueprints/DataTable/EventForDay` _returnvalue)) (`.Day_11_FD3FEA414E56BE98A9503E87627CA723` (break `/Game/Blueprints/DataTable/Parametrs` (`self.GetParametrs`))))
          (`KismetArrayLibrary.Array_Add` (`/Game/Blueprints/GI_GameInstance.EventsForCurrentDay` _gameinst) _array_element)
          (set `/Game/Blueprints/GI_GameInstance.CurrentEvent` 0 _gameinst))))))

(fn `SetupLettersForDay`
  (`KismetArrayLibrary.Array_Clear` (`self.LettersForCurrentDay`))
  (bind _outrownames (`DataTableFunctionLibrary.GetDataTableRowNames` "/Game/Blueprints/DataTable/Letters.Letters"))
  (for _array_element _outrownames
    (bind _returnvalue (`|GetDataTableRow` "/Game/Blueprints/DataTable/Letters.Letters" _array_element)
      (:`then`
        (if (== (`.Day_12_FD4168B84AD11D139CC06EB32DA6AFBD` (break `/Game/Blueprints/DataTable/Letter` _returnvalue)) (`.Day_11_FD3FEA414E56BE98A9503E87627CA723` (break `/Game/Blueprints/DataTable/Parametrs` (`self.GetParametrs`))))
          (`KismetArrayLibrary.Array_Add` (`self.LettersForCurrentDay`) _array_element))))))

(fn `UserConstructionScript`
  (bind _asgi_game_instance (cast `/Game/Blueprints/GI_GameInstance` (`GameplayStatics.GetGameInstance`)))
  (bind _output_get (set `self.GameInst` _asgi_game_instance))
  (`/Game/Blueprints/GI_GameInstance.InitGame` _output_get))